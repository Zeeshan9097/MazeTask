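; Procedural maze actor that builds a seeded, tile-based maze on a grid rounded to even dimensions.
; GenerateMaze uses randomized depth-first backtracking, carving cells two tiles apart with bridge tiles between and recording dead ends.
; The construction script places tiles through InstanceManeger: green for dead ends, dirt for paths, raised test meshes elsewhere.
; BeginPlay picks a new random seed, regenerates and adds path tiles to a hierarchical instanced static mesh.
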(event `self.ReceiveBeginPlay`
  (bind _tilessize (`self.TilesSize`))
  (bind _output_get (set `self.Seed` (`KismetMathLibrary.RandomIntegerInRange` 0 20)))
  (bind _pathtilesout (`self.GenerateMaze` _output_get (`self.Size`)))
  (bind _result (`BlueprintSetLibrary.Set_ToArray` _pathtilesout))
  (for _array_element _result
    (bind (_x _y) (break `IntPoint` _array_element))
    (`InstancedStaticMeshComponent.AddInstance` (`self.HierarchicalInstancedStaticMesh`) (`KismetMathLibrary.MakeTransform` (`KismetMathLibrary.MakeVector` (* _x _tilessize) (* _y _tilessize))) true)))

(fn `AddNeighbourLoc`
  (params (F_Size :type "IntPoint Structure (by ref)") (`Random Stream` :type "RandomStream Structure (by ref)") (currentLoc :type "IntPoint Structure (by ref)") (PathTiles :type "Set of IntPoint Structure (by ref)") (BridgeTiles :type "Set of IntPoint Structure (by ref)") (ToCheck :type "Set of IntPoint Structure (by ref)") (EndPAths :type "Set of IntPoint Structure (by ref)"))
  (locals (Neighbourindex :type Integer))
  (bind (_floor _bridge) (`self.GetNeighbourAnd Bridge` (`local.currentLoc`) (`local.Neighbourindex`)))
  (bind _returnvalue (+ (`local.Neighbourindex`) 1))
  (set `local.Neighbourindex` (`KismetMathLibrary.RandomIntegerInRangeFromStream` 0 3 (`local.Random Stream`)))
  (if (`self.CheckIfValidLoc` (`self.GetNeighbourAnd Bridge` (`local.currentLoc`) (`local.Neighbourindex`)) (`local.F_Size`) (`local.PathTiles`) (`local.BridgeTiles`)) :!label _label
    (`BlueprintSetLibrary.Set_Add` (`local.PathTiles`) _floor)
    (`BlueprintSetLibrary.Set_Add` (`local.BridgeTiles`) _bridge)
    (`BlueprintSetLibrary.Set_Add` (`local.ToCheck`) _floor)
    (`self.AddNeighbourLoc` (`local.F_Size`) (`local.Random Stream`) _floor (`local.PathTiles`) (`local.BridgeTiles`) (`local.ToCheck`) (`local.EndPAths`))
    (else
      (`/Game/BluePrints/CustumMacLib.DoN+` 4
        (:`Exist`
          (set `local.Neighbourindex` (`KismetMathLibrary.SelectInt` 0 _returnvalue (>= _returnvalue 4)))
          (goto _label))
        (:`OverNth`
          (bind _count (`self.GetNeighbourCount` (`local.currentLoc`) (`local.PathTiles`)))
          (if (== _count 1)
            (`BlueprintSetLibrary.Set_Add` (`local.EndPAths`) (`local.currentLoc`))))))))

(fn `BackTrack`
  (params (CurrentTiles :type "IntPoint Structure (by ref)") (ToCheck :type "Set of IntPoint Structure (by ref)") (BridgeTiles :type "Set of IntPoint Structure (by ref)") (PathTiles :type "Set of IntPoint Structure (by ref)"))
  (bind _result (`BlueprintSetLibrary.Set_ToArray` ToCheck))
  (bind _output (`|GetArrayItem` _result (`KismetArrayLibrary.Array_LastIndex` _result)))
  (`|VariableSetRef` (`local.CurrentTiles`) _output)
  (`BlueprintSetLibrary.Set_Remove` (`local.ToCheck`) _output)
  (bind _result_2 (`BlueprintSetLibrary.Set_ToArray` (`local.BridgeTiles`)))
  (bind _output_2 (`|GetArrayItem` _result_2 (`KismetArrayLibrary.Array_LastIndex` _result_2)))
  (`BlueprintSetLibrary.Set_Add` (`local.PathTiles`) _output_2)
  (`BlueprintSetLibrary.Set_Remove` (`local.BridgeTiles`) _output_2))

(fn `GenerateMaze`
  (params (Seed :type Integer) (Size :type "IntPoint Structure"))
  (returns (PathTilesOUT :type "Set of IntPoint Structure") (EndPAthsOUT :type "Set of IntPoint Structure"))
  (locals (RandomStream :type "RandomStream Structure") (L_Size :type "IntPoint Structure") (StartingLoc :type "IntPoint Structure") (CurrentLoc :type "IntPoint Structure") (PathTiles :type "Set of IntPoint Structure") (BridgeTiles :type "Set of IntPoint Structure") (ToCheck :type "Set of IntPoint Structure") (EndPAths :type "Set of IntPoint Structure"))
  (`KismetMathLibrary.SetRandomStreamSeed` (`local.RandomStream`) Seed)
  (set `local.L_Size` Size)
  (bind _output_get (set `local.StartingLoc` (`self.GetRandomLocInBLock` (`local.L_Size`) (`local.RandomStream`))))
  (set `local.CurrentLoc` _output_get)
  (`self.AddNeighbourLoc` (`local.L_Size`) (`local.RandomStream`) (`local.CurrentLoc`) (`local.PathTiles`) (`local.BridgeTiles`) (`local.ToCheck`) (`local.EndPAths`) :!label _label)
  (if (> (`BlueprintSetLibrary.Set_Length` (`local.ToCheck`)) 0)
    (`self.BackTrack` (`local.CurrentLoc`) (`local.ToCheck`) (`local.BridgeTiles`) (`local.PathTiles`))
    (goto _label)
    (else
      (return (`local.PathTiles`) (`local.EndPAths`)))))

(fn `GetNeighbourCount`
  (params (CurrentLoc :type "IntPoint Structure (by ref)") (PathTiles :type "Set of IntPoint Structure (by ref)"))
  (returns (Count :type Integer))
  (locals (counter :type Integer))
  (for _array_element (`self.getNeighbourLoc` CurrentLoc 1)
    (if (`BlueprintSetLibrary.Set_Contains` (`local.PathTiles`) _array_element)
      (`/Engine/EditorBlueprintResources/StandardMacros.IncrementInt` (`local.counter`))))
  (return (`local.counter`)))

(fn `spwanMazeMesh`
  (locals (LoopLoc :type "IntPoint Structure") (loopIndex :type Integer) (segementIndex :type "Array of Boolean"))
  (bind (_size_x _size_y) (break `IntPoint` (`self.Size`)))
  (for _index (range (+ _size_x 1))
    (for _index_2 (range (+ _size_y 1))
      (set `local.LoopLoc` (make `IntPoint` _index _index_2))
      (if (`BlueprintSetLibrary.Set_Contains` (`self.Path Tiles`) (`local.LoopLoc`))
        (message `/Game/BluePrints/BPi_intanceManeger.AddNewMeshintance` (`self.instanceManeger`) (select `bool` (`BlueprintSetLibrary.Set_Contains` (`self.End PAths`) (`local.LoopLoc`)) :`false` "/Game/Meshes/DirtGroundTile.DirtGroundTile" :`true` "/Game/Meshes/GreenGroundTile.GreenGroundTile" :!type "StaticMesh Object Reference") (`self.BuilTilesLoc` (`local.LoopLoc`)))
        (for (_array_element _array_index) (`self.getNeighbourLoc` (`local.LoopLoc`) 1)
          (set `local.loopIndex` _array_index)
          (bind _returnvalue (`BlueprintSetLibrary.Set_Contains` (`self.Path Tiles`) _array_element))
          (`KismetArrayLibrary.Array_Set` (`local.segementIndex`) (`local.loopIndex`) _returnvalue true)
          (if _returnvalue
            _))
        (else
          (message `/Game/BluePrints/BPi_intanceManeger.AddNewMeshintance` (`self.instanceManeger`) "/Game/TestMesh.TestMesh" (`self.BuilTilesLoc` (`local.LoopLoc`) 800.0)))))))

(fn `UserConstructionScript`
  (bind (_size_x _size_y) (break `IntPoint` (`self.Size`)))
  (message `/Game/BluePrints/BPi_intanceManeger.RemoveAllintance\`` (`self.instanceManeger`))
  (set `self.Size` (make `IntPoint` (* (/ _size_x 2) 2) (* (/ _size_y 2) 2)))
  (bind (_pathtilesout _endpathsout) (`self.GenerateMaze` (`self.Seed`) (`self.Size`)))
  (set `self.Path Tiles` _pathtilesout)
  (set `self.End PAths` _endpathsout)
  (`self.spwanMazeMesh`))