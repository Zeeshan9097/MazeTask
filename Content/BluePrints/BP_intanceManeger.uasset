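; BP_intanceManeger is an actor that manages instanced static meshes, grouping all instances of the same mesh under one component.
; AddNewMeshintance lazily creates a Hierarchical Instanced Static Mesh component per mesh, caches it in the InstanceCompnentList map, and returns the world-space instance's index.
; Other functions remove one instance by index or clear one or all meshes' instances, keeping the components.
; Single-instance removal does not check that the mesh is registered.
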(fn `AddNewMeshintance`
  (params (Mesh :type "StaticMesh Object Reference") (Transform :type "Transform Structure"))
  (returns (`bSuccessfull?` :type Boolean) (index :type Integer))
  (bind (_value _returnvalue) (`BlueprintMapLibrary.Map_Find` (`self.InstanceCompnentList`) (`local.Mesh`)))
  (if _returnvalue
    (bind _returnvalue_2 (`InstancedStaticMeshComponent.AddInstance` _value (`local.Transform`) true))
    (return true _returnvalue_2)
    (else
      (bind _returnvalue_3 (`AddComponent|NODE_AddHierarchicalInstancedStaticMeshComponent-0`))
      (`BlueprintMapLibrary.Map_Add` (`self.InstanceCompnentList`) (`local.Mesh`) _returnvalue_3)
      (`StaticMeshComponent.SetStaticMesh` _returnvalue_3 (`local.Mesh`))
      (bind _returnvalue_4 (`InstancedStaticMeshComponent.AddInstance` _returnvalue_3 (`local.Transform`) true))
      (return true _returnvalue_4))))

(fn `AllMeshRemoveintqance`
  (params (Mesh :type "StaticMesh Object Reference"))
  (returns (`bSuccessfull?` :type Boolean))
  (bind (_value _returnvalue) (`BlueprintMapLibrary.Map_Find` (`self.InstanceCompnentList`) (`local.Mesh`)))
  (if _returnvalue
    (`InstancedStaticMeshComponent.ClearInstances` _value)
    (return true)
    (else
      (return false))))

(fn `RemoveAllintance\``
  (returns (`bSuccessfull?` :type Boolean))
  (bind _keys (`BlueprintMapLibrary.Map_Keys` (`self.InstanceCompnentList`)))
  (for _array_element _keys
    (`InstancedStaticMeshComponent.ClearInstances` (`BlueprintMapLibrary.Map_Find` (`self.InstanceCompnentList`) _array_element)))
  (return true))

(fn `RemoveMeshintance`
  (params (Mesh :type "StaticMesh Object Reference") (index :type Integer))
  (returns (`bSuccessfull?` :type Boolean))
  (if true
    (bind _returnvalue (`InstancedStaticMeshComponent.RemoveInstance` (`BlueprintMapLibrary.Map_Find` (`self.InstanceCompnentList`) (`local.Mesh`)) (`local.index`)))
    (return _returnvalue)
    (else
      (return false))))

(fn `UserConstructionScript`)